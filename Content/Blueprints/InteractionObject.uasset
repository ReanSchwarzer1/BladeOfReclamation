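; InteractionObject is an interactable actor that shows a text widget when the player presses Interact near it.
; Box overlap with Pawn_TwoHanded toggles the actor's input, creating a widget with InteractionText and opening a gate on entry, closing it on exit.
; BeginPlay runs the same widget creation and gate opening.
; Interact passes through the gate to add the widget to the viewport, followed by a delay that leads nowhere.
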(event `self.ReceiveBeginPlay`
  (bind _returnvalue (`|CreateWidget` "/Game/Blueprints/InteractionWidget.InteractionWidget_C" :!label _label))
  (set `/Game/Blueprints/InteractionWidget.InteractionText` (`self.Interaction Text`) _returnvalue)
  (goto _label_2 :!via `Open`))

(event `self.Box.OnComponentBeginOverlap`
  (params (OverlappedComponent :type "PrimitiveComponent Object Reference") (OtherActor :type "Actor Object Reference") (OtherComp :type "PrimitiveComponent Object Reference") (OtherBodyIndex :type Integer) (bFromSweep :type Boolean) (SweepResult :type "HitResult Structure (by ref)"))
  (cast `/Game/BladesOfRec/Blueprints/Pawn_TwoHanded` OtherActor)
  (`self.EnableInput` (`GameplayStatics.GetPlayerController` 0))
  (goto _label))

(event `self.Box.OnComponentEndOverlap`
  (params (OverlappedComponent :type "PrimitiveComponent Object Reference") (OtherActor :type "Actor Object Reference") (OtherComp :type "PrimitiveComponent Object Reference") (OtherBodyIndex :type Integer))
  (cast `/Game/BladesOfRec/Blueprints/Pawn_TwoHanded` OtherActor)
  (`self.DisableInput` (`GameplayStatics.GetPlayerController` 0))
  (goto _label_2 :!via `Close`))

(event `InputAction|Interact`
  (params (Key :type "Key Structure"))
  (:`Pressed`
    (`/Engine/EditorBlueprintResources/StandardMacros.Gate` true :!label _label_2
      (:`Exit`
        (`UserWidget.AddToViewport` (stale `self.ReceiveBeginPlay` _returnvalue) 0)
        (`KismetSystemLibrary.Delay` 1.0)))))

(fn `UserConstructionScript`)